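; BP_VoidBall is a ball actor that launches from the player's camera and flags BallAlive on BP_Character during its lifetime.
; CalculateRute line-traces forward by BallDistance, then a timeline lerps position and drives sphere scale toward the hit point, or the maximum-range point.
; Sphere overlap freezes updates only on the hit path.
; Ten seconds after the timeline finishes, it clears BallAlive and destroys itself.
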(event `/Game/BluePrints/Interface_VoidBall.CalculateRute`
  (bind _asbp_character (cast `/Game/BluePrints/Character/BP_Character` (`GameplayStatics.GetPlayerPawn` 0)))
  (set `/Game/BluePrints/Character/BP_Character.BallAlive?` true _asbp_character)
  (bind _cameracomp (`MyCharacter.CameraComp` _asbp_character))
  (bind _returnvalue (`SceneComponent.K2_GetComponentLocation` _cameracomp))
  (bind _output_get (set `self.vectorpos` _returnvalue))
  (bind _returnvalue_2 (+ _returnvalue (* (`KismetMathLibrary.GetForwardVector` (`SceneComponent.K2_GetComponentRotation` _cameracomp)) (`/Game/BluePrints/Character/BP_Character.ball_distance` _asbp_character))))
  (set `self.fwpos` _returnvalue_2)
  (bind (_outhit _returnvalue_3) (`KismetSystemLibrary.LineTraceSingle` _output_get _returnvalue_2 "TraceTypeQuery1"))
  (if _returnvalue_3
    (bind (_direction _newtrack_0 _newtrack_2) (`Timeline|Timeline_0` :!via `PlayFromStart`)
      (:`Update`
        (if (not (`self.stop?`))
          (`SceneComponent.SetWorldScale3D` (`self.Sphere`) (`KismetMathLibrary.Conv_DoubleToVector` _newtrack_2))
          (`self.K2_SetActorLocation` (`KismetMathLibrary.VLerp` (`self.vectorpos`) (`.Location` (`GameplayStatics.BreakHitResult` _outhit)) _newtrack_0))))
      (:`Finished`
        (set `self.stop?` false)
        (`KismetSystemLibrary.Delay` 10.0)
        (set `/Game/BluePrints/Character/BP_Character.BallAlive?` false _asbp_character)
        (`self.K2_DestroyActor`)))
    (else
      (bind (_direction_2 _newtrack_0_2 _newtrack_1) (`Timeline|Timeline_1` :!via `PlayFromStart`)
        (:`Update`
          (`SceneComponent.SetWorldScale3D` (`self.Sphere`) (`KismetMathLibrary.Conv_DoubleToVector` _newtrack_1))
          (`self.K2_SetActorLocation` (`KismetMathLibrary.VLerp` (`self.vectorpos`) (`self.fwpos`) _newtrack_0_2)))
        (:`Finished`
          (set `self.stop?` false)
          (`KismetSystemLibrary.Delay` 10.0)
          (set `/Game/BluePrints/Character/BP_Character.BallAlive?` false _asbp_character)
          (`self.K2_DestroyActor`))))))

(event `self.Sphere.OnComponentBeginOverlap`
  (params (OverlappedComponent :type "PrimitiveComponent Object Reference") (OtherActor :type "Actor Object Reference") (OtherComp :type "PrimitiveComponent Object Reference") (OtherBodyIndex :type Integer) (bFromSweep :type Boolean) (SweepResult :type "HitResult Structure (by ref)"))
  (set `self.stop?` true))

(fn `UserConstructionScript`)