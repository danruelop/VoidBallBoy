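; BP_ButtonPuzzle is a pressure-plate puzzle button that reports its pressed state to a linked object.
; Overlapping Trigger sets ButtonPressed and plays Timeline_0, which reverses once Trigger has no overlapping actors.
; Timeline updates set the button's relative location from its own transform with a zero offset.
; When the timeline finishes, it swaps the pressed or red material and calls ActiveMessage on ObjectToSelect with the state.
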(event `self.Trigger.OnComponentBeginOverlap`
  (params (OverlappedComponent :type "PrimitiveComponent Object Reference") (OtherActor :type "Actor Object Reference") (OtherComp :type "PrimitiveComponent Object Reference") (OtherBodyIndex :type Integer) (bFromSweep :type Boolean) (SweepResult :type "HitResult Structure (by ref)"))
  (bind _buttonpuzzle (`self.ButtonPuzzle`))
  (bind _buttonpuzzle_2 (`self.ButtonPuzzle`))
  (if (not (`self.ButtonPressed`))
    (set `self.ButtonPressed` true)
    (`KismetSystemLibrary.PrintString` "Dentro")
    (`Timeline|Timeline_0` :!label _label
      (:`Update`
        (`SceneComponent.K2_SetRelativeLocation` _buttonpuzzle (`KismetMathLibrary.TransformLocation` (`SceneComponent.GetRelativeTransform` _buttonpuzzle)) false false))
      (:`Finished`
        (if (`self.ButtonPressed`)
          (`PrimitiveComponent.SetMaterial` _buttonpuzzle_2 0 "/Game/BluePrints/BP_ButtonPuzzle/M_ButtonPressed.M_ButtonPressed")
          (else
            (`PrimitiveComponent.SetMaterial` _buttonpuzzle_2 0 "/Game/Assets/Materials/Colors/MI_Lit_Red.MI_Lit_Red")))
        (message `/Game/BluePrints/BP_ButtonPuzzle/BPI_Activate.Active` (`self.ObjectToSelect`) (`self.ButtonPressed`))))))

(event `self.Trigger.OnComponentEndOverlap`
  (params (OverlappedComponent :type "PrimitiveComponent Object Reference") (OtherActor :type "Actor Object Reference") (OtherComp :type "PrimitiveComponent Object Reference") (OtherBodyIndex :type Integer))
  (if (not (`KismetArrayLibrary.Array_IsValidIndex` (`PrimitiveComponent.GetOverlappingActors` (`self.Trigger`) null)))
    (set `self.ButtonPressed` false)
    (`KismetSystemLibrary.PrintString` "Fuera")
    (goto _label :!via `Reverse`)))

(fn `UserConstructionScript`)