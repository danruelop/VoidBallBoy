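; Controllable ring for the button puzzle that spins through a RotatingMovement component, which is deactivated at BeginPlay.
; RotationActive starts the spin when passed true, but only prints a debug message when passed false.
; Stopping is deferred to Tick, which deactivates the movement once rotation is off and the root's pitch is near -90 degrees, intended as the initial position.
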(event `/Game/BluePrints/BP_ButtonPuzzle/BPI_Rotate.RotationActive`
  (params (IsRotating :type Boolean))
  (if IsRotating
    (`KismetSystemLibrary.PrintString` "Activado")
    (`ActorComponent.Activate` (`self.RotatingMovement`) false)
    (else
      (`KismetSystemLibrary.PrintString` "Desactivado"))))

(event `self.ReceiveBeginPlay`
  (`ActorComponent.Deactivate` (`self.RotatingMovement`) :!label _label))

(event `self.ReceiveTick`
  (params (DeltaSeconds :type "Float (single-precision)"))
  (bind (_relativerotation_roll _relativerotation_pitch) (`KismetMathLibrary.BreakRotator` (`SceneComponent.RelativeRotation` (`self.DefaultSceneRoot`))))
  ;[1 1 1] Esperar a que vuelva a la posición inicial
  (bind _returnvalue (not (stale `/Game/BluePrints/BP_ButtonPuzzle/BPI_Rotate.RotationActive` IsRotating)))
  (if _returnvalue
    (if (>= -89.0 _relativerotation_pitch)
      (if (<= -91.0 _relativerotation_pitch)
        (if _returnvalue
          (goto _label))))))

(fn `UserConstructionScript`)