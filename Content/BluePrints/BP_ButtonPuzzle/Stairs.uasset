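; Stairs actor for the button puzzle with a Portal component that ends the game when the player touches it.
; On a Portal hit, it checks that the other actor is the player's BP_Character.
; It then shows the EndWidget with mouse cursor and game-and-UI input, pauses the game and plays a 2D music track.
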(event `self.Portal.OnComponentHit`
  (params (HitComponent :type "PrimitiveComponent Object Reference") (OtherActor :type "Actor Object Reference") (OtherComp :type "PrimitiveComponent Object Reference") (NormalImpulse :type "Vector Structure") (Hit :type "HitResult Structure (by ref)"))
  (bind _returnvalue (`GameplayStatics.GetPlayerController` 0))
  (bind _asbp_character (cast `/Game/BluePrints/Character/BP_Character` (`GameplayStatics.GetPlayerCharacter` 0)))
  (if (== OtherActor _asbp_character)
    (bind _returnvalue_2 (`|CreateWidget` "/Game/BluePrints/BP_ButtonPuzzle/EndWidget.EndWidget_C"))
    (`UserWidget.AddToViewport` _returnvalue_2 0)
    (set `PlayerController.bShowMouseCursor` true _returnvalue)
    (`WidgetBlueprintLibrary.SetInputMode_GameAndUIEx` _returnvalue null)
    (`GameplayStatics.SetGamePaused` true)
    (`GameplayStatics.PlaySound2D` "/Game/Assets/Sounds/MUSIC_voidball-startmenu-loop.MUSIC_voidball-startmenu-loop" 1.0 1.0 0.0 null null)))

(fn `UserConstructionScript`)