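; BP_ButtonPuzzle3 is a pressure button for a puzzle that switches rotation on a linked object while something occupies its trigger.
; The first overlap sets ButtonPressed and the pressed material, and the button releases to red only once no actors remain overlapping.
; Each state change prints a debug string and passes ButtonPressed to ObjectToSelect through RotationActiveMessage.
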(event `self.Trigger.OnComponentBeginOverlap`
  (params (OverlappedComponent :type "PrimitiveComponent Object Reference") (OtherActor :type "Actor Object Reference") (OtherComp :type "PrimitiveComponent Object Reference") (OtherBodyIndex :type Integer) (bFromSweep :type Boolean) (SweepResult :type "HitResult Structure (by ref)"))
  (if (not (`self.ButtonPressed`))
    (set `self.ButtonPressed` true)
    (`KismetSystemLibrary.PrintString` "Dentro")
    (`PrimitiveComponent.SetMaterial` (`self.ButtonPuzzle`) 0 "/Game/BluePrints/BP_ButtonPuzzle/M_ButtonPressed.M_ButtonPressed")
    (message `/Game/BluePrints/BP_ButtonPuzzle/BPI_Rotate.RotationActive` (`self.ObjectToSelect`) (`self.ButtonPressed`) :!label _label)))

(event `self.Trigger.OnComponentEndOverlap`
  (params (OverlappedComponent :type "PrimitiveComponent Object Reference") (OtherActor :type "Actor Object Reference") (OtherComp :type "PrimitiveComponent Object Reference") (OtherBodyIndex :type Integer))
  (if (not (`KismetArrayLibrary.Array_IsValidIndex` (`PrimitiveComponent.GetOverlappingActors` (`self.Trigger`) null)))
    (set `self.ButtonPressed` false)
    (`KismetSystemLibrary.PrintString` "Fuera")
    (`PrimitiveComponent.SetMaterial` (`self.ButtonPuzzle`) 0 "/Game/Assets/Materials/Colors/MI_Lit_Red.MI_Lit_Red")
    (goto _label)))

(fn `UserConstructionScript`)