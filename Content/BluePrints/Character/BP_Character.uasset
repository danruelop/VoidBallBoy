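; Player character Blueprint with a slot-based inventory and a void ball ability.
; BeginPlay adds the main HUD and initializes an anchored inventory grid; debug inputs add or remove BlueKey and Cube items looked up in the Items_DT data table.
; Fire plays a montage, spawns BP_VoidBall ahead of the camera and calls its CalculateRuteMessage, with BallAlive blocking further casts; this graph never clears that flag.
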(event `InputAction|Add`
  (params (Key :type "Key Structure"))
  ;[1 1 1] ADD ITEM
  (:`Pressed`
    (`KismetSystemLibrary.PrintString` "Test: Adding Item")
    (bind _returnvalue (`|GetDataTableRow` "/Game/BluePrints/Inventario/DataTables/Items_DT.Items_DT" "BlueKey")
      (:`then`
        (`/Game/BluePrints/Inventario/Libraries/Inventory_BPFL.AddItem` _returnvalue)))))

(event `InputAction|Remove`
  (params (Key :type "Key Structure"))
  ;[1 1 1] remove item
  (:`Pressed`
    (`KismetSystemLibrary.PrintString` "Test: Removing Item")
    (bind _returnvalue (`|GetDataTableRow` "/Game/BluePrints/Inventario/DataTables/Items_DT.Items_DT" "BlueKey")
      (:`then`
        (`/Game/BluePrints/Inventario/Libraries/Inventory_BPFL.RemoveItem` _returnvalue)))))

(event `InputAction|Add1`
  (params (Key :type "Key Structure"))
  ;[1 1 1] ADD ITEM
  (:`Pressed`
    (`KismetSystemLibrary.PrintString` "Test: Adding Item")
    (bind _returnvalue (`|GetDataTableRow` "/Game/BluePrints/Inventario/DataTables/Items_DT.Items_DT" "Cube")
      (:`then`
        (`/Game/BluePrints/Inventario/Libraries/Inventory_BPFL.AddItem` _returnvalue)))))

(event `InputAction|Remove1`
  (params (Key :type "Key Structure"))
  ;[1 1 1] remove item
  (:`Pressed`
    (`KismetSystemLibrary.PrintString` "Test: Removing Item")
    (bind _returnvalue (`|GetDataTableRow` "/Game/BluePrints/Inventario/DataTables/Items_DT.Items_DT" "Cube")
      (:`then`
        (`/Game/BluePrints/Inventario/Libraries/Inventory_BPFL.RemoveItem` _returnvalue)))))

(event `self.ReceiveBeginPlay`
  ;[1 1 1] Comment
  (bind _returnvalue (`|CreateWidget` "/Game/BluePrints/Inventario/Main_HUD_WG.Main_HUD_WG_C"))
  (`UserWidget.AddToViewport` _returnvalue 0)
  (`/Game/BluePrints/Inventario/Libraries/Inventory_BPFL.InitializeInventory` 9 (make `Anchors` (0.86 0.6) (0.97 0.9))))

(event `InputAction|Fire`
  (params (Key :type "Key Structure"))
  (bind _camera (`self.Camera`))
  (bind _returnvalue (`SceneComponent.K2_GetComponentRotation` _camera))
  (:`Pressed`
    (if (not (`self.BallAlive?`))
      (set `self.BallAlive?` true)
      (`AnimInstance.Montage_Play` (`SkeletalMeshComponent.GetAnimInstance` (`self.Mesh`)) "/Game/BluePrints/Character/Anim/Animation/MagicHealMontage.MagicHealMontage" 1.0 "MontageLength" 0.0 true)
      (bind _returnvalue_2 (`|SpawnActorFromClass` "/Game/BluePrints/VoidBall/BP_VoidBall.BP_VoidBall_C" (`KismetMathLibrary.MakeTransform` (+ (`SceneComponent.K2_GetComponentLocation` _camera) (* (`KismetMathLibrary.GetForwardVector` _returnvalue) (`self.ball_distance`))) _returnvalue (0.5 0.5 0.5)) "Undefined" "OverrideRootScale" null null))
      (message `/Game/BluePrints/VoidBall/Interface_VoidBall.CalculateRute` _returnvalue_2))))

(fn `UserConstructionScript`)