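; Enemy turret that activates when the player enters its Sphere, changing eye colour and light and sounding an alert.
; A timeline turns the head toward the player and gates projectile fire through a FireRate delay.
; AbsorbEnemies lets a VoidBall pull the head in on Tick, scaling it by distance until its DeadZone destroys the turret and decrements the absorbed-item counter.
; A CRing overlap triggers a delayed explosion and destruction.
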(event `self.ReceiveBeginPlay`
  (set `self.InitialScale` (`SceneComponent.K2_GetComponentScale` (`self.EnemyHead`)))
  (if (`self.isCamo`)
    (`PrimitiveComponent.SetMaterial` (`self.EnemyHead`) 0 "/Game/Assets/dspace.dspace")))

(event `self.ReceiveTick`
  (params (DeltaSeconds :type "Float (single-precision)"))
  (bind _enemyhead (`self.EnemyHead`))
  (bind _enemyhead_2 (`self.EnemyHead`))
  ;[1 1 1] Enemy Absorption
  (`/Engine/EditorBlueprintResources/StandardMacros.IsValid` (stale `/Game/BluePrints/VoidBall/Interface_VoidBall.AbsorbEnemies` _VoidBall)
    (:`Is Valid`
      (set `self.F_actualDistance` (`KismetMathLibrary.Vector_Distance` (`SceneComponent.K2_GetComponentLocation` (`Actor.RootComponent` (stale `/Game/BluePrints/VoidBall/Interface_VoidBall.AbsorbEnemies` _output_get))) (`SceneComponent.K2_GetComponentLocation` _enemyhead)))
      (bind _asinventory_gi (cast `/Game/BluePrints/Inventory_GI` (`GameplayStatics.GetGameInstance`)))
      (`PrimitiveComponent.SetPhysicsLinearVelocity` _enemyhead (* (`KismetMathLibrary.GetForwardVector` (`KismetMathLibrary.FindLookAtRotation` (`SceneComponent.K2_GetComponentLocation` _enemyhead) (`SceneComponent.K2_GetComponentLocation` (`/Game/BluePrints/VoidBall/BP_VoidBall.Horizont` (`self.VoidBall`))))) (`/Game/BluePrints/Inventory_GI.absorptionForce` _asinventory_gi)) false "None")
      (`SceneComponent.SetWorldScale3D` _enemyhead_2 (* (`self.InitialScale`) (/ (`self.F_actualDistance`) (`self.F_initialDistance`))))
      (if (`PrimitiveComponent.IsOverlappingComponent` (`/Game/BluePrints/VoidBall/BP_VoidBall.DeadZone` (`self.VoidBall`)) _enemyhead_2)
        (bind _asinventory_gi_2 (cast `/Game/BluePrints/Inventory_GI` (`GameplayStatics.GetGameInstance`)))
        (set `/Game/BluePrints/Inventory_GI.absorbedItemCounter` (- (`/Game/BluePrints/Inventory_GI.absorbedItemCounter` _asinventory_gi_2) 1) _asinventory_gi_2)
        (`self.K2_DestroyActor`)))))

(event `/Game/BluePrints/VoidBall/Interface_VoidBall.AbsorbEnemies`
  (params (_VoidBall :type "/Game/BluePrints/VoidBall/BP_VoidBall Object Reference"))
  ;[1 1 1] Enemy Absorption
  (bind _output_get (set `self.VoidBall` _VoidBall))
  (set `self.F_initialDistance` (`KismetMathLibrary.Vector_Distance` (`SceneComponent.K2_GetComponentLocation` (`Actor.RootComponent` _output_get)) (`SceneComponent.K2_GetComponentLocation` (`self.EnemyHead`)))))

(event `self.Sphere.OnComponentBeginOverlap`
  (params (OverlappedComponent :type "PrimitiveComponent Object Reference") (OtherActor :type "Actor Object Reference") (OtherComp :type "PrimitiveComponent Object Reference") (OtherBodyIndex :type Integer) (bFromSweep :type Boolean) (SweepResult :type "HitResult Structure (by ref)"))
  (if (== OtherActor (`GameplayStatics.GetPlayerCharacter` 0))
    (`self.Activate`)))

(event `self.Sphere.OnComponentEndOverlap`
  (params (OverlappedComponent :type "PrimitiveComponent Object Reference") (OtherActor :type "Actor Object Reference") (OtherComp :type "PrimitiveComponent Object Reference") (OtherBodyIndex :type Integer))
  (if (== OtherActor (`GameplayStatics.GetPlayerCharacter` 0))
    (`self.Deactivate`)))

(event `Activate`
  (`self.UpdateEyeColour` (`self.ActivateEyeColour`) 5000.0)
  (set `self.Activated?` true)
  (`GameplayStatics.SpawnSoundAtLocation` "/Game/Assets/Sounds/Danger1.Danger1" (`self.K2_GetActorLocation`) (struct) 0.7 1.0 0.0 null null)
  (`Timeline|CombatTimeline` :!label _label
    (:`Update`
      (`|ExecutionSequence`
        (:`then_0`
          (`self.UpdateRotationToLookAtPlayer`))
        (:`then_1`
          (`KismetSystemLibrary.Delay` (`self.FireRate`))
          (if (`self.Activated?`)
            (`self.SpawnProjectileAtPlayer`)))))))

(event `Deactivate`
  (`self.UpdateEyeColour` (`self.DeactivateEyeColour`) 1000.0)
  (set `self.Activated?` false)
  (goto _label :!via `Stop`))

(event `self.Sphere1.OnComponentBeginOverlap`
  (params (OverlappedComponent :type "PrimitiveComponent Object Reference") (OtherActor :type "Actor Object Reference") (OtherComp :type "PrimitiveComponent Object Reference") (OtherBodyIndex :type Integer) (bFromSweep :type Boolean) (SweepResult :type "HitResult Structure (by ref)"))
  ;[1 1 1] Die if struck by ring
  (if (== OtherActor (`self.cRing`))
    (`KismetSystemLibrary.PrintString` "F")
    (`KismetSystemLibrary.Delay` 2.0)
    (`GameplayStatics.SpawnEmitterAttached` (`self.explosion`) (`self.Eye`) "ExplosionPoint" (0.0 0.0 0.0) (struct) (* (`SceneComponent.K2_GetComponentScale` (`self.ParticleSystem`)) 3))
    (`KismetSystemLibrary.Delay` 0.5)
    (`self.K2_DestroyActor`)))

(fn `SpawnProjectileAtPlayer`
  (bind (_returnvalue_location _returnvalue_rotation) (`KismetMathLibrary.BreakTransform` (`SceneComponent.K2_GetComponentToWorld` (`self.SpawnPoint`))))
  (bind _returnvalue (`|SpawnActorFromClass` "/Game/BluePrints/BP_EnemyTurret/Projectiles.Projectiles_C" (`KismetMathLibrary.MakeTransform` _returnvalue_location _returnvalue_rotation) "Undefined" "OverrideRootScale" null null))
  (bind _staticmesh (`/Game/BluePrints/BP_EnemyTurret/Projectiles.StaticMesh` _returnvalue))
  (`PrimitiveComponent.SetPhysicsLinearVelocity` _staticmesh (* (`KismetMathLibrary.GetDirectionUnitVector` (`SceneComponent.K2_GetComponentLocation` (`self.SpawnPoint`)) (`self.K2_GetActorLocation` (`GameplayStatics.GetPlayerCharacter` 0))) (`self.ProjectileSpeed`)) false "None")
  (bind _returnvalue_2 (`PrimitiveComponent.CreateDynamicMaterialInstance` _staticmesh 0 "/Game/BluePrints/BP_EnemyTurret/ProximityTurretEye.ProximityTurretEye" "None"))
  (`MaterialInstanceDynamic.SetVectorParameterValue` _returnvalue_2 "Colour" (`self.ActivateEyeColour`))
  (`GameplayStatics.SpawnSoundAtLocation` "/Game/Assets/Sounds/Laser1.Laser1" (`SceneComponent.K2_GetComponentLocation` (`self.SpawnPoint`)) (struct) 1.0 0.5 0.0 null null))

(fn `UpdateEyeColour`
  (params (Colour :type "LinearColor Structure") (NewIntensity :type "Float (double-precision)"))
  (`MaterialInstanceDynamic.SetVectorParameterValue` (`self.DynamicEyeMaterial`) "Colour" Colour)
  (`LightComponent.SetLightColor` (`self.Light`) Colour true)
  (`LightComponent.SetIntensity` (`self.Light`) NewIntensity))

(fn `UpdateRotationToLookAtPlayer`
  (`SceneComponent.K2_SetWorldRotation` (`self.EnemyHead`) (`KismetMathLibrary.RLerp` (`SceneComponent.K2_GetComponentRotation` (`self.EnemyHead`)) (`KismetMathLibrary.FindLookAtRotation` (`SceneComponent.K2_GetComponentLocation` (`self.EnemyHead`)) (`self.K2_GetActorLocation` (`GameplayStatics.GetPlayerCharacter` 0))) 0.5 true) false false))

(fn `UserConstructionScript`
  ;[1 1 1] Eye Material
  (bind _returnvalue (`PrimitiveComponent.CreateDynamicMaterialInstance` (`self.Eye`) 0 "/Game/BluePrints/BP_EnemyTurret/ProximityTurretEye.ProximityTurretEye" "None"))
  (bind _output_get (set `self.DynamicEyeMaterial` _returnvalue))
  (`MaterialInstanceDynamic.SetVectorParameterValue` _output_get "Colour" (`self.DeactivateEyeColour`))
  ;[1 1 1] Eye colour
  (`LightComponent.SetLightColor` (`self.Light`) (`self.DeactivateEyeColour`) true))