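; Enemy turret projectile that damages the player character and explodes on impact.
; When its static mesh hits something, it subtracts Damage from BP_Character's Health if that actor is the player, then calls CheckPlayerHealthMessage on the character.
; It then spawns an explosion effect and sound at the mesh location and destroys itself, provided the player pawn casts to BP_Character.
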(event `self.StaticMesh.OnComponentHit`
  (params (HitComponent :type "PrimitiveComponent Object Reference") (OtherActor :type "Actor Object Reference") (OtherComp :type "PrimitiveComponent Object Reference") (NormalImpulse :type "Vector Structure") (Hit :type "HitResult Structure (by ref)"))
  (bind _returnvalue (`SceneComponent.K2_GetComponentLocation` (`self.StaticMesh`)))
  (bind _asbp_character (cast `/Game/BluePrints/Character/BP_Character` (`GameplayStatics.GetPlayerCharacter` 0)))
  (if (== _asbp_character OtherActor)
    (set `/Game/BluePrints/Character/BP_Character.health` (- (`/Game/BluePrints/Character/BP_Character.health` _asbp_character) (`self.Damage`)) _asbp_character)
    (message `/Game/BluePrints/VoidBall/Interface_VoidBall.CheckPlayerHealth` _asbp_character))
  (`GameplayStatics.SpawnEmitterAtLocation` "/Game/StarterContent/Particles/P_Explosion.P_Explosion" _returnvalue)
  (`GameplayStatics.SpawnSoundAtLocation` "/Game/StarterContent/Audio/Explosion01.Explosion01" _returnvalue (struct) 0.7 1.0 0.0 null null)
  (`self.K2_DestroyActor`))

(fn `UserConstructionScript`)