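; Proximity turret that raises its neck, tracks the player and fires projectiles while the player is inside its sphere trigger.
; Overlap events move the neck with a looping lerp, switch the eye material and light colour, and start or stop CombatTimeline.
; Timeline updates smoothly rotate the head toward the player, while a FireRate Delay paces shots.
; Projectiles launch by physics velocity at the player, tinted with the active eye colour.
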(event `self.Sphere.OnComponentBeginOverlap`
  (params (OverlappedComponent :type "PrimitiveComponent Object Reference") (OtherActor :type "Actor Object Reference") (OtherComp :type "PrimitiveComponent Object Reference") (OtherBodyIndex :type Integer) (bFromSweep :type Boolean) (SweepResult :type "HitResult Structure (by ref)"))
  (if (== OtherActor (`GameplayStatics.GetPlayerCharacter` 0))
    (`self.Activate`)))

(event `self.Sphere.OnComponentEndOverlap`
  (params (OverlappedComponent :type "PrimitiveComponent Object Reference") (OtherActor :type "Actor Object Reference") (OtherComp :type "PrimitiveComponent Object Reference") (OtherBodyIndex :type Integer))
  (if (== OtherActor (`GameplayStatics.GetPlayerCharacter` 0))
    (`self.Deactivate`)))

(event `Activate`
  (`self.MoveNeckPosition` (0.0 0.0 50.0)
    (:`End`
      (`self.UpdateEyeColour` (`self.ActivateEyeColour`))
      (set `self.Activated?` true)
      (`GameplayStatics.SpawnSoundAtLocation` "/Game/Assets/Sounds/Danger1.Danger1" (`self.K2_GetActorLocation`) (struct) 0.7 1.0 0.0 null null)
      (`Timeline|CombatTimeline` :!label _label
        (:`Update`
          (`|ExecutionSequence`
            (:`then_0`
              (`self.UpdateRotationToLookAtPlayer`))
            (:`then_1`
              (`KismetSystemLibrary.Delay` (`self.FireRate`))
              (if (`self.Activated?`)
                (`self.SpawnProjectileAtPlayer`)))))))))

(event `Deactivate`
  (`self.MoveNeckPosition` (0.0 0.0 -50.0)
    (:`End`
      (`self.UpdateEyeColour` (`self.DeactivateEyeColour`))
      (set `self.Activated?` false)
      (goto _label :!via `Stop`))))

(fn `SpawnProjectileAtPlayer`
  (bind (_returnvalue_location _returnvalue_rotation) (`KismetMathLibrary.BreakTransform` (`SceneComponent.K2_GetComponentToWorld` (`self.SpawnPoint`))))
  (bind _returnvalue (`|SpawnActorFromClass` "/Game/BluePrints/BP_EnemyTurret/Projectiles.Projectiles_C" (`KismetMathLibrary.MakeTransform` _returnvalue_location _returnvalue_rotation) "Undefined" "OverrideRootScale" null null))
  (bind _staticmesh (`/Game/BluePrints/BP_EnemyTurret/Projectiles.StaticMesh` _returnvalue))
  (`PrimitiveComponent.SetPhysicsLinearVelocity` _staticmesh (* (`KismetMathLibrary.GetDirectionUnitVector` (`SceneComponent.K2_GetComponentLocation` (`self.SpawnPoint`)) (`self.K2_GetActorLocation` (`GameplayStatics.GetPlayerCharacter` 0))) (`self.ProjectileSpeed`)) false "None")
  (bind _returnvalue_2 (`PrimitiveComponent.CreateDynamicMaterialInstance` _staticmesh 0 "/Game/BluePrints/BP_EnemyTurret/ProximityTurretEye.ProximityTurretEye" "None"))
  (`MaterialInstanceDynamic.SetVectorParameterValue` _returnvalue_2 "Colour" (`self.ActivateEyeColour`))
  (`GameplayStatics.SpawnSoundAtLocation` "/Game/Assets/Sounds/Laser1.Laser1" (`SceneComponent.K2_GetComponentLocation` (`self.SpawnPoint`)) (struct) 1.0 0.5 0.0 null null))

(fn `UpdateEyeColour`
  (params (Colour :type "LinearColor Structure"))
  (`MaterialInstanceDynamic.SetVectorParameterValue` (`self.DynamicEyeMaterial`) "Colour" Colour)
  (`LightComponent.SetLightColor` (`self.Light`) Colour true))

(fn `UpdateRotationToLookAtPlayer`
  (`SceneComponent.K2_SetWorldRotation` (`self.Head`) (`KismetMathLibrary.RLerp` (`SceneComponent.K2_GetComponentRotation` (`self.Head`)) (`KismetMathLibrary.FindLookAtRotation` (`SceneComponent.K2_GetComponentLocation` (`self.Head`)) (`self.K2_GetActorLocation` (`GameplayStatics.GetPlayerCharacter` 0))) 0.5 true) false false))

(fn `UserConstructionScript`
  ;[1 1 1] Body Material
  (`PrimitiveComponent.SetMaterial` (`self.Body`) 0 (`self.BodyMaterial`))
  (`PrimitiveComponent.SetMaterial` (`self.Neck`) 0 (`self.BodyMaterial`))
  (`PrimitiveComponent.SetMaterial` (`self.Head`) 0 (`self.BodyMaterial`))
  ;[1 1 1] Eye Material
  (bind _returnvalue (`PrimitiveComponent.CreateDynamicMaterialInstance` (`self.Eye`) 0 "/Game/BluePrints/BP_EnemyTurret/ProximityTurretEye.ProximityTurretEye" "None"))
  (bind _output_get (set `self.DynamicEyeMaterial` _returnvalue))
  (`MaterialInstanceDynamic.SetVectorParameterValue` _output_get "Colour" (`self.DeactivateEyeColour`))
  ;[1 1 1] Eye colour
  (`LightComponent.SetLightColor` (`self.Light`) (`self.DeactivateEyeColour`) true))