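; BP_FallDeath is a trigger volume that handles the player's death when MyCharacter overlaps it.
; On overlap it plays a sound, shows a FadeToBlack widget and destroys the BP_VoidBall if the Inventory_GI game instance flags it alive.
; It then pauses the game and opens DeathScreenWidget with UI-only input and a visible cursor.
; The construction script sizes the Overlap box from BoxExtension.
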(event `self.Overlap.OnComponentBeginOverlap`
  (params (OverlappedComponent :type "PrimitiveComponent Object Reference") (OtherActor :type "Actor Object Reference") (OtherComp :type "PrimitiveComponent Object Reference") (OtherBodyIndex :type Integer) (bFromSweep :type Boolean) (SweepResult :type "HitResult Structure (by ref)"))
  (bind _returnvalue (`GameplayStatics.GetPlayerController` 0))
  (cast `MyCharacter` OtherActor)
  (`GameplayStatics.SpawnSound2D` "/Game/Assets/Sounds/SFX_SEEN1.SFX_SEEN1" 0.4 1.0 0.0 null)
  (bind _returnvalue_2 (`|CreateWidget` "/Game/BluePrints/CheckpointSystem/FadeToBlack.FadeToBlack_C"))
  (`/Game/BluePrints/CheckpointSystem/FadeToBlack.FadeToBlack` _returnvalue_2)
  (`UserWidget.AddToViewport` _returnvalue_2 0)
  (bind _asinventory_gi (cast `/Game/BluePrints/Inventory_GI` (`GameplayStatics.GetGameInstance`)))
  (if (`/Game/BluePrints/Inventory_GI.B_isVoidBallAlive?` _asinventory_gi)
    (bind _returnvalue_3 (`GameplayStatics.GetActorOfClass` "/Game/BluePrints/VoidBall/BP_VoidBall.BP_VoidBall_C"))
    (`self.K2_DestroyActor` _returnvalue_3))
  (`GameplayStatics.SetGamePaused` true)
  (bind _returnvalue_4 (`|CreateWidget` "/Game/MainMenu/DeathScreenWidget.DeathScreenWidget_C"))
  (message `/Game/BluePrints/VoidBall/Interface_VoidBall.deathMusic` _returnvalue_4)
  (`UserWidget.AddToViewport` _returnvalue_4 0)
  (`WidgetBlueprintLibrary.SetInputMode_UIOnlyEx` _returnvalue null)
  (set `PlayerController.bShowMouseCursor` true _returnvalue))

(fn `UserConstructionScript`
  (`BoxComponent.SetBoxExtent` (`self.Overlap`) (`self.BoxExtension`) true))