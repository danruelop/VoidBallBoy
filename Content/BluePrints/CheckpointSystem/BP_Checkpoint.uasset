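; BP_Checkpoint is a checkpoint actor that saves the player's respawn point when MyCharacter overlaps it.
; On overlap it loads the CheckpointSaveGame from its slot, or creates one if none exists.
; It stores a transform 200 units above the actor with zero rotation, writes the save, and shows a SavedWidget notification on screen.
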(event `self.Overlap.OnComponentBeginOverlap`
  (params (OverlappedComponent :type "PrimitiveComponent Object Reference") (OtherActor :type "Actor Object Reference") (OtherComp :type "PrimitiveComponent Object Reference") (OtherBodyIndex :type Integer) (bFromSweep :type Boolean) (SweepResult :type "HitResult Structure (by ref)"))
  (bind _returnvalue_location (`KismetMathLibrary.BreakTransform` (`self.GetTransform`)))
  (cast `MyCharacter` OtherActor)
  ;[1 1 1] UpdateSaveCheckpoint
  (bind _returnvalue (`GameplayStatics.DoesSaveGameExist` (`self.CheckpointSaveName`)))
  (if _returnvalue
    (bind _returnvalue_2 (`GameplayStatics.LoadGameFromSlot` (`self.CheckpointSaveName`)))
    (bind _ascheckpoint_save_game (cast `/Game/BluePrints/CheckpointSystem/CheckpointSaveGame` _returnvalue_2))
    (set `self.SaveGameReference` _ascheckpoint_save_game)
    (else
      (bind _returnvalue_3 (`GameplayStatics.CreateSaveGameObject` "/Game/BluePrints/CheckpointSystem/CheckpointSaveGame.CheckpointSaveGame_C"))
      (set `self.SaveGameReference` _returnvalue_3)))
  (set `/Game/BluePrints/CheckpointSystem/CheckpointSaveGame.Checkpoint` (`KismetMathLibrary.MakeTransform` (+ _returnvalue_location (0.0 0.0 200.0))) (`self.SaveGameReference`))
  (`GameplayStatics.SaveGameToSlot` (`self.SaveGameReference`) (`self.CheckpointSaveName`))
  (bind _returnvalue_4 (`|CreateWidget` "/Game/BluePrints/CheckpointSystem/SavedWidget.SavedWidget_C"))
  (`/Game/BluePrints/CheckpointSystem/SavedWidget.DisplaySaveNotification` _returnvalue_4)
  (`UserWidget.AddToViewport` _returnvalue_4 0))

(fn `UserConstructionScript`)