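; BP_CardTerminal is a keycard terminal that unlocks a door with the inventory card named by CardNameColor.
; BeginPlay enables input and tints the hologram screen for BlueKey or YellowKey.
; Overlapping InsertCardZone shows an interaction widget and opens a Gate for the Action input.
; Pressing Action flashes the widget, removes the card, and, if found, plays a sound, destroys DoorToOpen and activates MovableDoor's InterpToMovement when valid.
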(event `self.ReceiveBeginPlay`
  (bind _cardnamecolor (`self.cardNameColor`))
  (`self.EnableInput` (`GameplayStatics.GetPlayerController` 0))
  (if (== _cardnamecolor "BlueKey")
    ;[1 1 1] Change color by name
    (`PrimitiveComponent.SetMaterial` (`self.ScreenText_GreaterThan2`) 0 "/Game/BluePrints/Inventario/HologramBlue.HologramBlue")
    (`PrimitiveComponent.SetMaterial` (`self.ScreenText_Line`) 0 "/Game/BluePrints/Inventario/HologramBlue.HologramBlue")
    (`PrimitiveComponent.SetMaterial` (`self.ScreenText_GreaterThan1`) 0 "/Game/BluePrints/Inventario/HologramBlue.HologramBlue")
    (`TextRenderComponent.SetTextRenderColor` (`self.UpperScreenText`) (`self.blue`))
    (elif (== _cardnamecolor "YellowKey")
      (`PrimitiveComponent.SetMaterial` (`self.ScreenText_GreaterThan2`) 0 "/Game/BluePrints/Inventario/HologramYellow.HologramYellow")
      (`PrimitiveComponent.SetMaterial` (`self.ScreenText_Line`) 0 "/Game/BluePrints/Inventario/HologramYellow.HologramYellow")
      (`PrimitiveComponent.SetMaterial` (`self.ScreenText_GreaterThan1`) 0 "/Game/BluePrints/Inventario/HologramYellow.HologramYellow")
      (`TextRenderComponent.SetTextRenderColor` (`self.UpperScreenText`) (`self.yellow`)))))

(event `InputAction|Action` :consume false
  (params (Key :type "Key Structure"))
  (bind _movabledoor (`self.movableDoor`))
  (bind _doortoopen (`self.doorToOpen`))
  (:`Pressed`
    (if (`PrimitiveComponent.IsOverlappingActor` (`self.InsertCardZone`) (stale `self.InsertCardZone.OnComponentBeginOverlap` OtherActor))
      (set `/Game/BluePrints/BP_CardTerminal/InteractionWidget.IsPressed` true (stale `self.InsertCardZone.OnComponentBeginOverlap` _returnvalue))
      (`KismetSystemLibrary.Delay` 0.2)
      (set `/Game/BluePrints/BP_CardTerminal/InteractionWidget.IsPressed` false (stale `self.InsertCardZone.OnComponentBeginOverlap` _returnvalue))
      (`/Engine/EditorBlueprintResources/StandardMacros.Gate` true :!label _label
        (:`Exit`
          (bind (_founditem _amountfound _slot _iteminfo) (`/Game/BluePrints/Inventario/Libraries/Inventory_BPFL.ScanForItem` (`self.cardNameColor`)))
          (`/Game/BluePrints/Inventario/Libraries/Inventory_BPFL.RemoveItem` _iteminfo)
          (if _founditem
            (`GameplayStatics.PlaySoundAtLocation` "/Game/Assets/Sounds/door_open.door_open" (`SceneComponent.K2_GetComponentLocation` (`StaticMeshActor.StaticMeshComponent` _doortoopen)) (struct) 1.0 1.0 0.0 null null null)
            (`self.K2_DestroyActor` _doortoopen)
            (if (`KismetSystemLibrary.IsValid` _movabledoor)
              (`ActorComponent.Activate` (`/Game/BluePrints/BP_Obstacle/BP_movableDoor.InterpToMovement` _movabledoor) false))))))))

(event `self.InsertCardZone.OnComponentBeginOverlap`
  (params (OverlappedComponent :type "PrimitiveComponent Object Reference") (OtherActor :type "Actor Object Reference") (OtherComp :type "PrimitiveComponent Object Reference") (OtherBodyIndex :type Integer) (bFromSweep :type Boolean) (SweepResult :type "HitResult Structure (by ref)"))
  (cast `MyCharacter` OtherActor)
  (bind _returnvalue (`|CreateWidget` "/Game/BluePrints/BP_CardTerminal/InteractionWidget.InteractionWidget_C"))
  (`UserWidget.AddToViewport` _returnvalue 0)
  (goto _label :!via `Open`))

(event `self.InsertCardZone.OnComponentEndOverlap`
  (params (OverlappedComponent :type "PrimitiveComponent Object Reference") (OtherActor :type "Actor Object Reference") (OtherComp :type "PrimitiveComponent Object Reference") (OtherBodyIndex :type Integer))
  (cast `MyCharacter` OtherActor)
  (`Widget.RemoveFromParent` (stale `self.InsertCardZone.OnComponentBeginOverlap` _returnvalue))
  (goto _label :!via `Close`))

(fn `UserConstructionScript`)