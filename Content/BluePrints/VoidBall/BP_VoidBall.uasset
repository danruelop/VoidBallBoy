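; BP_VoidBall is a thrown void orb that grows and triggers absorption on nearby enemy turrets.
; CalculateRute traces from the player camera up to BallDistance, stopping short of any hit by a size-based offset.
; Timelines lerp the ball to that point and scale it up with a sound.
; It then enables AbsorptionLimit collision, messages overlapping turrets, waits, clears the game instance alive flag and destroys itself.
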(event `/Game/BluePrints/VoidBall/Interface_VoidBall.CalculateRute`
  (bind _absorptionlimit (`self.AbsorptionLimit`))
  (bind _absorptionlimit_2 (`self.AbsorptionLimit`))
  (bind _asbp_character (cast `/Game/BluePrints/Character/BP_Character` (`GameplayStatics.GetPlayerPawn` 0)))
  (set `self.BP_Character` _asbp_character)
  (set `self.V_ballscale` (`SceneComponent.K2_GetComponentScale` (`self.Sphere`)))
  (bind _camera (`/Game/BluePrints/Character/BP_Character.Camera` _asbp_character))
  (bind _returnvalue (`SceneComponent.K2_GetComponentLocation` _camera))
  (bind _output_get (set `self.V_origin` _returnvalue))
  (bind _output_get_2 (set `self.V_distance` (+ _returnvalue (* (`KismetMathLibrary.GetForwardVector` (`SceneComponent.K2_GetComponentRotation` _camera)) (`/Game/BluePrints/Character/BP_Character.ball_distance` _asbp_character)))))
  (bind (_outhit _returnvalue_2) (`KismetSystemLibrary.LineTraceSingle` :`Start` _output_get :`End` _output_get_2 :`TraceChannel` "TraceTypeQuery1" :`DrawDebugType` "ForDuration"))
  (if _returnvalue_2
    (set `self.V_final` (+ (`self.V_origin`) (* (`KismetMathLibrary.GetForwardVector` (`SceneComponent.K2_GetComponentRotation` _camera)) (- (`.Distance` (`GameplayStatics.BreakHitResult` _outhit)) (* 55.0 (`self.F_maxsize`))))))
    (bind (_direction _newtrack_1) (`Timeline|Timeline_0` :!via `PlayFromStart`)
      (:`Update`
        (`self.K2_SetActorLocation` (`KismetMathLibrary.VLerp` (`self.V_origin`) (`self.V_final`) _newtrack_1)))
      (:`Finished`
        (`GameplayStatics.SpawnSoundAtLocation` "/Game/Assets/Sounds/Broly_Omega_Blaster_Sound_Effect_5.Broly_Omega_Blaster_Sound_Effect_5" (`self.K2_GetActorLocation`) (struct) 1.0 1.0 0.0 null null)
        (bind (_direction_2 _newtrack_0) (`Timeline|Timeline_3` :!via `PlayFromStart`)
          (:`Update`
            (`SceneComponent.SetWorldScale3D` (`self.Sphere`) (+ (`self.V_ballscale`) (* _newtrack_0 (`self.F_maxsize`)))))
          (:`Finished`
            (bind _returnvalue_3 (`GameplayStatics.GetActorOfClass` "/Game/BluePrints/EnemyTurret/BP_EnemyTurret.BP_EnemyTurret_C"))
            (`PrimitiveComponent.SetCollisionEnabled` _absorptionlimit_2 "QueryAndPhysics")
            (bind _sphere (`/Game/BluePrints/EnemyTurret/BP_EnemyTurret.Sphere` _returnvalue_3))
            (`PrimitiveComponent.IgnoreComponentWhenMoving` _absorptionlimit_2 _sphere true)
            (`PrimitiveComponent.IgnoreComponentWhenMoving` _sphere _absorptionlimit_2 true)
            (for _array_element (`PrimitiveComponent.GetOverlappingActors` (`self.AbsorptionLimit`) "/Game/BluePrints/EnemyTurret/BP_EnemyTurret.BP_EnemyTurret_C")
              (message `/Game/BluePrints/VoidBall/Interface_VoidBall.Absorption` _array_element self))
            (`KismetSystemLibrary.Delay` 3.5)
            (bind _asinventory_gi (cast `/Game/BluePrints/Inventory_GI` (`GameplayStatics.GetGameInstance`)))
            (set `/Game/BluePrints/Inventory_GI.B_isVoidBallAlive?` false _asinventory_gi)
            (`self.K2_DestroyActor`)))))
    (else
      (bind (_direction_3 _newtrack_0_2) (`Timeline|Timeline_1` :!via `PlayFromStart`)
        (:`Update`
          (`self.K2_SetActorLocation` (`KismetMathLibrary.VLerp` (`self.V_origin`) (`self.V_distance`) _newtrack_0_2)))
        (:`Finished`
          (`GameplayStatics.SpawnSoundAtLocation` "/Game/Assets/Sounds/Broly_Omega_Blaster_Sound_Effect_5.Broly_Omega_Blaster_Sound_Effect_5" (`self.K2_GetActorLocation`) (struct) 1.0 1.0 0.0 null null)
          (bind (_direction_4 _newtrack_0_3) (`Timeline|Timeline_2` :!via `PlayFromStart`)
            (:`Update`
              (`SceneComponent.SetWorldScale3D` (`self.Sphere`) (+ (`self.V_ballscale`) (* _newtrack_0_3 (`self.F_maxsize`)))))
            (:`Finished`
              (bind _returnvalue_4 (`GameplayStatics.GetActorOfClass` "/Game/BluePrints/EnemyTurret/BP_EnemyTurret.BP_EnemyTurret_C"))
              (`PrimitiveComponent.SetCollisionEnabled` _absorptionlimit "QueryAndPhysics")
              (bind _sphere_2 (`/Game/BluePrints/EnemyTurret/BP_EnemyTurret.Sphere` _returnvalue_4))
              (`PrimitiveComponent.IgnoreComponentWhenMoving` _absorptionlimit _sphere_2 true)
              (`PrimitiveComponent.IgnoreComponentWhenMoving` _sphere_2 _absorptionlimit true)
              (for _array_element_2 (`PrimitiveComponent.GetOverlappingActors` (`self.AbsorptionLimit`) "/Game/BluePrints/EnemyTurret/BP_EnemyTurret.BP_EnemyTurret_C")
                (message `/Game/BluePrints/VoidBall/Interface_VoidBall.Absorption` _array_element_2 self))
              (`KismetSystemLibrary.Delay` 3.5)
              (bind _asinventory_gi_2 (cast `/Game/BluePrints/Inventory_GI` (`GameplayStatics.GetGameInstance`)))
              (set `/Game/BluePrints/Inventory_GI.B_isVoidBallAlive?` false _asinventory_gi_2)
              (`self.K2_DestroyActor`))))))))

(fn `UserConstructionScript`)