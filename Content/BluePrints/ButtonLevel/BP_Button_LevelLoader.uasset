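; Interactable button, derived from a parent button Blueprint, that loads the level named in LevelToLoad0.
; Overlap of MyCharacter with the box shows an interaction widget and opens a Gate, while leaving removes the widget and closes it.
; The Interact input briefly flags the widget as pressed, then, through the open Gate, runs the parent interaction and opens the level after a short delay.
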(event `self.ReceiveBeginPlay`
  (bind (_returnvalue_location _returnvalue_rotation _returnvalue_scale) (`KismetMathLibrary.BreakTransform` (`SceneComponent.GetRelativeTransform` (`self.Button`))))
  (set `self.Out Position` (`KismetMathLibrary.MakeTransform` _returnvalue_location _returnvalue_rotation _returnvalue_scale))
  (set `self.In Position` (`KismetMathLibrary.MakeTransform` _returnvalue_location _returnvalue_rotation _returnvalue_scale))
  (`self.EnableInput` (`GameplayStatics.GetPlayerController` 0)))

(event `InputAction|Interact`
  (params (Key :type "Key Structure"))
  (:`Pressed`
    (set `/Game/BluePrints/ButtonLevel/InteractionWidget.IsPressed` true (stale `self.BoxCollision.OnComponentBeginOverlap` _returnvalue))
    (`KismetSystemLibrary.Delay` 0.2)
    (set `/Game/BluePrints/ButtonLevel/InteractionWidget.IsPressed` false (stale `self.BoxCollision.OnComponentBeginOverlap` _returnvalue))
    (`/Engine/EditorBlueprintResources/StandardMacros.Gate` true :!label _label
      (:`Exit`
        (`parent.Interact`)
        (`KismetSystemLibrary.Delay` 0.5)
        (if (!= (`self.LevelToLoad_0`) "None")
          (`GameplayStatics.OpenLevel` (`self.LevelToLoad_0`)))))))

(event `self.BoxCollision.OnComponentBeginOverlap`
  (params (OverlappedComponent :type "PrimitiveComponent Object Reference") (OtherActor :type "Actor Object Reference") (OtherComp :type "PrimitiveComponent Object Reference") (OtherBodyIndex :type Integer) (bFromSweep :type Boolean) (SweepResult :type "HitResult Structure (by ref)"))
  (cast `MyCharacter` OtherActor)
  (bind _returnvalue (`|CreateWidget` "/Game/BluePrints/ButtonLevel/InteractionWidget.InteractionWidget_C"))
  (`UserWidget.AddToViewport` _returnvalue 0)
  (goto _label :!via `Open`))

(event `self.BoxCollision.OnComponentEndOverlap`
  (params (OverlappedComponent :type "PrimitiveComponent Object Reference") (OtherActor :type "Actor Object Reference") (OtherComp :type "PrimitiveComponent Object Reference") (OtherBodyIndex :type Integer))
  (cast `MyCharacter` OtherActor)
  (`Widget.RemoveFromParent` (stale `self.BoxCollision.OnComponentBeginOverlap` _returnvalue))
  (goto _label :!via `Close`))

(fn `UserConstructionScript`
  (`parent.UserConstructionScript`))