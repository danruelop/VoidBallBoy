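; Enemy AI Blueprint that wanders, chases the player and plays an attack montage, using a Tick-driven IDLE/Chase/Attack state machine that starts in Chase.
; Horizontal distance and a line-of-sight trace drive transitions, with delayed give-up to IDLE and pawn sensing to resume Chase.
; Attack returns to Chase when out of range or whenever sight is clear.
; Void-ball absorption logic is disconnected, leaving its event empty.
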(event `self.ReceiveBeginPlay`
  ;[1 1 1] Beginplay (setup)
  (bind _asbp_character (cast `/Game/BluePrints/Character/BP_Character` (`GameplayStatics.GetPlayerCharacter` 0)))
  (set `self.MyPlayer` _asbp_character)
  (set `self.state` "NewEnumerator1"))

(event `/Game/BluePrints/VoidBall/Interface_VoidBall.Absorption`
  (params (_VoidBall :type "/Game/BluePrints/VoidBall/BP_VoidBall Object Reference"))
  ;[1 1 1] Enemy Absorption
)

(event `self.PawnSensing.OnSeePawn`
  (params (Pawn :type "Pawn Object Reference"))
  ;[1 1 1] Decision System
  ;;[1 1 1] IDLE State
  (cast `/Game/BluePrints/Character/BP_Character` Pawn)
  (if (`self.isPatchClear?`)
    (goto _label :!via `Open`)))

(event `CloseIDLE`
  ;[1 1 1] Decision System
  ;;[1 1 1] IDLE State
  (goto _label :!via `Close`))

(event `self.ReceiveTick`
  (params (DeltaSeconds :type "Float (single-precision)"))
  ;[1 1 1] Decision System
  (`|ExecutionSequence`
    (:`then_0`
      (switch `/Game/BluePrints/Enemy/States` (`self.state`)
        (:`NewEnumerator0`
          ;;[1 1 1] IDLE State
          (`self.IDLE`)
          (`/Engine/EditorBlueprintResources/StandardMacros.Gate` true :!label _label
            (:`Exit`
              (`self.changeState` "NewEnumerator1"))))
        (:`NewEnumerator1`
          ;;[1 1 1] Chase State
          (`self.Chase`)
          (`|ExecutionSequence`
            (:`then_0`
              (`self.CloseIDLE`))
            (:`then_1`
              (if (<= (`self.getDistanceToPlayer`) (`self.AttackRange`))
                (`self.changeState` "NewEnumerator2")
                (elif (not (`self.isPatchClear?`))
                  (`KismetSystemLibrary.Delay` (`self.giveUpTime`))
                  (`self.changeState` "NewEnumerator0"))))))
        (:`NewEnumerator2`
          ;;[1 1 1] Attack State
          (`self.Attack`)
          (`|ExecutionSequence`
            (:`then_0`
              (`self.CloseIDLE`))
            (:`then_1`
              (if (or (> (`self.getDistanceToPlayer`) (`self.AttackRange`)) (`self.isPatchClear?`))
                (`self.changeState` "NewEnumerator1")))))))))

(event `IDLE`
  ;[1 1 1] IDLE Action
  (`/Engine/EditorBlueprintResources/StandardMacros.DoOnce` false :!label _label_2
    (:`Completed`
      (`|AIMoveTo` self (`NavigationSystemV1.K2_GetRandomLocationInNavigableRadius` (`self.K2_GetActorLocation`) 999999.0 null null) null 300.0 true
        (:`OnSuccess`
          (`KismetSystemLibrary.Delay` (`self.IDLEPause`))
          (`self.resetIDLE`))))))

(event `resetIDLE`
  ;[1 1 1] IDLE Action
  (goto _label_2 :!via `Reset`))

(event `Chase`
  ;[1 1 1] Chase Action
  (`AIBlueprintHelperLibrary.SimpleMoveToActor` (`AIBlueprintHelperLibrary.GetAIController` self) (`self.MyPlayer`)))

(event `Attack`
  ;[1 1 1] Attack Action
  (`/Engine/EditorBlueprintResources/StandardMacros.DoOnce` false :!label _label_3
    (:`Completed`
      (`AnimInstance.Montage_Play` (`SkeletalMeshComponent.GetAnimInstance` (`self.Mesh`)) "/Game/BluePrints/Enemy/Animation/Enemy2/Animation/AN_Enemy2.AN_Enemy2" 1.0 "MontageLength" 0.0 true)
      (`KismetSystemLibrary.Delay` (`self.AttackRate`))
      (`self.ResetAttack`))))

(event `ResetAttack`
  ;[1 1 1] Attack Action
  (goto _label_3 :!via `Reset`))

(fn `changeState`
  (params (newState :type "/Game/BluePrints/Enemy/States Enum" :default "NewEnumerator0"))
  (`NavMovementComponent.StopActiveMovement` (`self.CharacterMovement`))
  (set `self.state` newState)
  (`self.resetIDLE`)
  (`self.ResetAttack`))

(fn `getDistanceToPlayer`
  (returns (distance :type "Float (double-precision)"))
  (bind (_returnvalue_x _returnvalue_y) (`KismetMathLibrary.BreakVector` (`self.K2_GetActorLocation`)))
  (bind (_returnvalue_x_2 _returnvalue_y_2) (`KismetMathLibrary.BreakVector` (`self.K2_GetActorLocation` (`self.MyPlayer`))))
  (return (`KismetMathLibrary.Sqrt` (+ (`KismetMathLibrary.Square` (- _returnvalue_x_2 _returnvalue_x)) (`KismetMathLibrary.Square` (- _returnvalue_y_2 _returnvalue_y))))))

(fn `isPatchClear?`
  (returns (`isClear?` :type Boolean))
  (bind _outhit (`KismetSystemLibrary.LineTraceSingle` :`Start` (`self.K2_GetActorLocation`) :`End` (`self.K2_GetActorLocation` (`self.MyPlayer`)) :`TraceChannel` "TraceTypeQuery2" :`DrawTime` 1.0))
  (cast `/Game/BluePrints/Character/BP_Character` (`.HitActor` (`GameplayStatics.BreakHitResult` _outhit))
    (:`then`
      (return true))
    (:`CastFailed`
      (return false))))

(fn `UserConstructionScript`)