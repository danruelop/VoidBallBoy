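; Example physics body that gets pulled into a VoidBall, shrinking as it approaches, then destroys itself.
; The Absorption event stores the VoidBall and the initial distance to it.
; While that reference is valid, Tick overrides the mesh's linear velocity toward the ball's Horizont component and scales TempABScale by current over initial distance.
; A Delay on Tick, marked as temporary, destroys the actor seconds after the pull starts.
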(event `self.ReceiveTick`
  (params (DeltaSeconds :type "Float (single-precision)"))
  (bind _staticmesh (`self.StaticMesh`))
  (`/Engine/EditorBlueprintResources/StandardMacros.IsValid` (stale `/Game/BluePrints/VoidBall/Interface_VoidBall.Absorption` _VoidBall)
    (:`Is Valid`
      (set `self.F_DistanceVB_AB` (`KismetMathLibrary.Vector_Distance` (`SceneComponent.K2_GetComponentLocation` (`Actor.RootComponent` (stale `/Game/BluePrints/VoidBall/Interface_VoidBall.Absorption` _output_get))) (`SceneComponent.K2_GetComponentLocation` (`self.StaticMesh`))))
      (`PrimitiveComponent.SetPhysicsLinearVelocity` _staticmesh (* (`KismetMathLibrary.GetForwardVector` (`KismetMathLibrary.FindLookAtRotation` (`SceneComponent.K2_GetComponentLocation` _staticmesh) (`SceneComponent.K2_GetComponentLocation` (`/Game/BluePrints/VoidBall/BP_VoidBall.Horizont` (`self.VoidBall`))))) 400.0) false "None")
      (`SceneComponent.SetWorldScale3D` (`self.StaticMesh`) (* (`self.Temp_AB_Scale`) (/ (`self.F_DistanceVB_AB`) (`self.f_initialDistance`))))
      ;[1 1 1] destruccion temporal
      (`KismetSystemLibrary.Delay` 3.0)
      (`self.K2_DestroyActor`))))

(event `/Game/BluePrints/VoidBall/Interface_VoidBall.Absorption`
  (params (_VoidBall :type "/Game/BluePrints/VoidBall/BP_VoidBall Object Reference"))
  (bind _output_get (set `self.VoidBall` _VoidBall))
  (set `self.f_initialDistance` (`KismetMathLibrary.Vector_Distance` (`SceneComponent.K2_GetComponentLocation` (`Actor.RootComponent` _output_get)) (`SceneComponent.K2_GetComponentLocation` (`self.StaticMesh`)))))

(fn `UserConstructionScript`)