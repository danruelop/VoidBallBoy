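; PickUp_BP is a world item pickup whose construction script loads its info and mesh from a data table row.
; Overlap with BP_Character shows an "[E]" nameplate and enables the Action input, which adds the item to inventory and destroys the actor on success.
; AbsorbItems sets a VoidBall that Tick pulls it toward by physics velocity, scaling it with distance.
; Reaching the DeadZone decrements the game instance's absorption counter and runs the same pickup.
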(event `self.ReceiveBeginPlay`
  (set `self.V_InitialScale` (`SceneComponent.K2_GetComponentScale` (`self.Model`)))
  (bind _aspick_up_name_plate_wg (cast `/Game/BluePrints/Inventario/Interactables/PickUpNamePlate_WG` (`WidgetComponent.GetUserWidgetObject` (`self.NamePlate`))))
  (`TextBlock.SetText` (`/Game/BluePrints/Inventario/Interactables/PickUpNamePlate_WG.NameText` _aspick_up_name_plate_wg) (`KismetTextLibrary.Conv_StringToText` (`KismetStringLibrary.Concat_StrStr` "[E] " (`KismetStringLibrary.Conv_NameToString` (`.Name_12_EEA559074776CFF92E1322A257F69596` (break `/Game/BluePrints/Inventario/Structures/Item_ST` (`self.information`))))))))

(event `self.InteractionCollider.OnComponentBeginOverlap`
  (params (OverlappedComponent :type "PrimitiveComponent Object Reference") (OtherActor :type "Actor Object Reference") (OtherComp :type "PrimitiveComponent Object Reference") (OtherBodyIndex :type Integer) (bFromSweep :type Boolean) (SweepResult :type "HitResult Structure (by ref)"))
  (if (`KismetMathLibrary.ClassIsChildOf` (`GameplayStatics.GetObjectClass` OtherActor) "/Game/BluePrints/Character/BP_Character.BP_Character_C")
    (`SceneComponent.SetVisibility` (`self.NamePlate`) true false)
    (`self.EnableInput` (`GameplayStatics.GetPlayerController` 0))))

(event `self.ReceiveTick`
  (params (DeltaSeconds :type "Float (single-precision)"))
  (bind _staticmesh (`self.StaticMesh`))
  ;[1 1 1] Item Absorption
  (`/Engine/EditorBlueprintResources/StandardMacros.IsValid` (stale `/Game/BluePrints/VoidBall/Interface_VoidBall.AbsorbItems` `Void Ball`)
    (:`Is Valid`
      (set `self.F actual distance` (`KismetMathLibrary.Vector_Distance` (`SceneComponent.K2_GetComponentLocation` (`Actor.RootComponent` (stale `/Game/BluePrints/VoidBall/Interface_VoidBall.AbsorbItems` _output_get))) (`SceneComponent.K2_GetComponentLocation` _staticmesh)))
      (`PrimitiveComponent.SetPhysicsLinearVelocity` _staticmesh (* (`KismetMathLibrary.GetForwardVector` (`KismetMathLibrary.FindLookAtRotation` (`SceneComponent.K2_GetComponentLocation` _staticmesh) (`SceneComponent.K2_GetComponentLocation` (`/Game/BluePrints/VoidBall/BP_VoidBall.Horizont` (`self.Void Ball`))))) 400.0) false "None")
      (`SceneComponent.SetWorldScale3D` (`self.StaticMesh`) (* (`self.V_InitialScale`) (/ (`self.F actual distance`) (`self.F initial distance`))))
      (if (`PrimitiveComponent.IsOverlappingComponent` (`/Game/BluePrints/VoidBall/BP_VoidBall.DeadZone` (`self.Void Ball`)) (`self.StaticMesh`))
        (bind _asinventory_gi (cast `/Game/BluePrints/Inventory_GI` (`GameplayStatics.GetGameInstance`)))
        (set `/Game/BluePrints/Inventory_GI.absorbedItemCounter` (- (`/Game/BluePrints/Inventory_GI.absorbedItemCounter` _asinventory_gi) 1) _asinventory_gi)
        (bind _added_ (`/Game/BluePrints/Inventario/Libraries/Inventory_BPFL.AddItem` (`self.information`) (`.Quantity_22_634D19C34B2875AB67450B9D038E47E5` (break `/Game/BluePrints/Inventario/Structures/Item_ST` (`self.information`))) :!label _label))
        (if _added_
          (`self.K2_DestroyActor`))))))

(event `/Game/BluePrints/VoidBall/Interface_VoidBall.AbsorbItems`
  (params (`Void Ball` :type "/Game/BluePrints/VoidBall/BP_VoidBall Object Reference"))
  ;[1 1 1] Item Absorption
  (bind _output_get (set `self.Void Ball` `Void Ball`))
  (set `self.F initial distance` (`KismetMathLibrary.Vector_Distance` (`SceneComponent.K2_GetComponentLocation` (`Actor.RootComponent` _output_get)) (`SceneComponent.K2_GetComponentLocation` (`self.StaticMesh`)))))

(event `self.InteractionCollider.OnComponentEndOverlap`
  (params (OverlappedComponent :type "PrimitiveComponent Object Reference") (OtherActor :type "Actor Object Reference") (OtherComp :type "PrimitiveComponent Object Reference") (OtherBodyIndex :type Integer))
  (if (`KismetMathLibrary.ClassIsChildOf` (`GameplayStatics.GetObjectClass` OtherActor) "/Game/BluePrints/Character/BP_Character.BP_Character_C")
    (`SceneComponent.SetVisibility` (`self.NamePlate`) false false)
    (`self.DisableInput` (`GameplayStatics.GetPlayerController` 0))))

(event `InputAction|Action`
  (params (Key :type "Key Structure"))
  ;[1 1 1] Item Absorption
  (:`Pressed`
    (goto _label)))

(fn `UserConstructionScript`
  (bind (_datatable _rowname) (break `DataTableRowHandle` (`self.item`)))
  (bind _returnvalue (`|GetDataTableRow` _datatable _rowname)
    (:`then`
      (set `self.information` _returnvalue)
      (`StaticMeshComponent.SetStaticMesh` (`self.Model`) (`.Model_19_DEE4C3644EA5860DA82ED78285DD0A4A` (break `/Game/BluePrints/Inventario/Structures/Item_ST` (`self.information`)))))))