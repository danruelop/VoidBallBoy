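; ActivatorPad is a one-shot pickup that switches on a linked jump pad when the void ball touches it.
; On sphere overlap with BP_VoidBall, it calls ActivatePad on the assigned BP_JumpPad, plays a 2D pickup sound and destroys itself.
; The construction script applies the configurable colour and intensity to a dynamic mesh material and matches the point light colour.
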(event `self.Sphere.OnComponentBeginOverlap`
  (params (OverlappedComponent :type "PrimitiveComponent Object Reference") (OtherActor :type "Actor Object Reference") (OtherComp :type "PrimitiveComponent Object Reference") (OtherBodyIndex :type Integer) (bFromSweep :type Boolean) (SweepResult :type "HitResult Structure (by ref)"))
  (cast `/Game/BluePrints/VoidBall/BP_VoidBall` OtherActor)
  (bind _asbp_jump_pad (cast `/Game/BluePrints/JumpPad/BP_JumpPad` (`self.JumpPadToActivate`)))
  (`/Game/BluePrints/JumpPad/BP_JumpPad.ActivatePad` _asbp_jump_pad)
  (`GameplayStatics.SpawnSound2D` "/Game/Assets/Sounds/pickup_Items.pickup_Items" 1.0 1.0 0.0 null)
  (`self.K2_DestroyActor`))

(fn `UserConstructionScript`
  (bind _returnvalue (`PrimitiveComponent.CreateDynamicMaterialInstance` (`self.StaticMesh`) 0 null "None"))
  (`MaterialInstanceDynamic.SetVectorParameterValue` _returnvalue "Colour" (`self.Colour`))
  (`MaterialInstanceDynamic.SetScalarParameterValue` _returnvalue "Intensity" (`self.Intensity`))
  (`LightComponent.SetLightColor` (`self.PointLight`) (`self.Colour`) true))