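; Player character Blueprint that fires a void ball projectile from the camera.
; On Fire press, if no ball is alive, it spawns a BP_VoidBall a set distance along the camera's forward vector, using the camera rotation and a configurable scale.
; The new ball then receives a CalculateRuteMessage call to compute its route.
; The file only reads the BallAlive flag and never sets it.
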(event `InputAction|Fire`
  (params (Key :type "Key Structure"))
  (bind _cameracomp (`self.CameraComp`))
  (bind _returnvalue (`SceneComponent.K2_GetComponentRotation` _cameracomp))
  (:`Pressed`
    (if (not (`self.BallAlive?`))
      (bind _returnvalue_2 (`|SpawnActorFromClass` "/Game/BluePrints/BP_VoidBall.BP_VoidBall_C" (`KismetMathLibrary.MakeTransform` (+ (`SceneComponent.K2_GetComponentLocation` _cameracomp) (* (`KismetMathLibrary.GetForwardVector` _returnvalue) (`self.ball_distance`))) _returnvalue (`self.ball_size`)) "Undefined" "OverrideRootScale" null null))
      (message `/Game/BluePrints/Interface_VoidBall.CalculateRute` _returnvalue_2))))

(fn `UserConstructionScript`)